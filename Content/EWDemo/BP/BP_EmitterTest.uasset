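; BP_EmitterTest is a test sound emitter for an acoustics demo, with input-driven play, stop and next-track controls over a sound list.
; On BeginPlay it sets early reflections on its AcousticsDetector and optionally starts delayed one-shot or timer-repeated playback.
; Tick can push the detector's reverb and room debug data to the shooter character's results widget.
; When moving, it orbits a center point, which follows the actor while grabbed via Interact.
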(event Custom|PlayByTimer
  (Audio|Components|Audio|Play (Variables|Default|GetAudioComponent) 0.0))

(event EventBeginPlay
  (bind _audiocomponent (Variables|Default|GetAudioComponent))
  (bind _timer (Variables|Default|GetTimer))
  (Class|AcousticsDetectorComponent|SetEarlyReflectionsEnabled (Variables|Default|GetAcousticsDetector) (Variables|Default|GetEnableReflections))
  (Variables|Default|SetCenter (Transformation|GetActorLocation))
  (if (Variables|Default|GetplaysAudio)
    (Utilities|FlowControl|Delay _timer)
    (Audio|Components|Audio|SetSound _audiocomponent (Utilities|Array|Get(acopy) (Variables|Default|GetEvent) (Variables|Default|GetcurAudioIdx)))
    (if (Variables|Default|GetisLoop)
      (Utilities|Time|SetTimerbyEvent (delegate Custom|PlayByTimer) _timer true)
      (else
        (Audio|Components|Audio|Play _audiocomponent 0.0)))))

(event EventStopInteract
  (Variables|Default|SetGrabbing false))

(event EventTick
  (params (DeltaSeconds :type Float%20%28single-precision%29))
  (bind _acousticsdetector (Variables|Default|GetAcousticsDetector))
  (bind _returnvalue (Class|AcousticsDetectorComponent|GetDebugOverlayData _acousticsdetector))
  (Utilities|FlowControl|Sequence
    (:then_0
      (if (Variables|Default|GetUpdateUI)
        (bind _asbp_shooter_character (Utilities|Casting|CastToBP_ShooterCharacter (Pawn|GetControlledPawn (Game|GetPlayerController 0))))
        (Default|SetParameters (Variables|/Game/EWDemo/UI/WBP_AcousticsDebugOverlay.WBP_AcousticsDebugOverlay_C|GetWBP_Values_Emitter (Variables|/Game/Variant_Shooter/Blueprints/BP_ShooterCharacter.BP_ShooterCharacter_C|GetResultsWidget _asbp_shooter_character)) (.close _returnvalue) (.mid _returnvalue) (.far _returnvalue) (.originalclose _returnvalue) (.originalmid _returnvalue) (.originalfar _returnvalue) (.outdoor _returnvalue) (.originaloutdoor _returnvalue) (.absorption _returnvalue) (.bisindoor _returnvalue) (.reverbenclosure _returnvalue) (.height _returnvalue) (.width _returnvalue) (.distancetolistener _returnvalue) (.reverbmultiplier _returnvalue) (.crossroomcontribution _returnvalue) "(Orange) Emitter")))
    (:then_1
      (if (Variables|Default|GetGrabbing)
        (Variables|Default|SetCenter (Transformation|GetActorLocation))
        (else
          ;[0.15 0.15 0.15 0.5] Movement
          (if (Variables|Default|GetisMoving)
            (bind _output_get (Variables|Default|SetOrbitAngleDeg%20 (+ (Variables|Default|GetOrbitAngleDeg%20) (* (Utilities|Time|GetWorldDeltaSeconds) (Variables|Default|GetMovementSpeed)))))
            (Transformation|SetActorLocation (Math|Vector|MakeVector (+ (* (Math|Trig|Cos(Radians) (Math|Trig|DegreesToRadians _output_get)) (Variables|Default|GetMovementRadius)) (.x (Variables|Default|GetCenter))) (+ (* (Math|Trig|Sin(Radians) (Math|Trig|DegreesToRadians _output_get)) (Variables|Default|GetMovementRadius)) (.y (Variables|Default|GetCenter))) (.z (Variables|Default|GetCenter))) false true)))))))

(event Input|ActionEvents|InputActionStopPlay
  (params (Key :type Key%20Structure :default "None"))
  (:Pressed
    (Variables|Default|SetplaysAudio false)
    (Audio|Components|Audio|Stop (Variables|Default|GetAudioComponent))))

(event Input|ActionEvents|InputActionPlay
  (params (Key :type Key%20Structure :default "None"))
  (bind _audiocomponent (Variables|Default|GetAudioComponent))
  (:Pressed
    (if (not (Variables|Default|GetplaysAudio))
      (Variables|Default|SetplaysAudio true)
      (Audio|Components|Audio|SetSound _audiocomponent (Utilities|Array|Get(acopy) (Variables|Default|GetEvent) (Variables|Default|GetcurAudioIdx)))
      (Audio|Components|Audio|Play _audiocomponent 0.0))))

(event Input|ActionEvents|InputActionNextAudio
  (params (Key :type Key%20Structure :default "None"))
  (bind _audiocomponent (Variables|Default|GetAudioComponent))
  (:Pressed
    (Utilities|FlowControl|Sequence
      (:then_0
        (Variables|Default|SetplaysAudio false)
        (Audio|Components|Audio|Stop _audiocomponent))
      (:then_1
        (bind _result (Math|Integer|IncrementInt (Variables|Default|GetcurAudioIdx))
          (:%20%20
            (bind _output_get (Variables|Default|SetcurAudioIdx _result))
            (if (>= _output_get (Utilities|Array|Length (Variables|Default|GetEvent)))
              (Variables|Default|SetcurAudioIdx 0))
            (Variables|Default|SetplaysAudio true)
            (Audio|Components|Audio|SetSound _audiocomponent (Utilities|Array|Get(acopy) (Variables|Default|GetEvent) (Variables|Default|GetcurAudioIdx)))
            (Audio|Components|Audio|Play _audiocomponent 0.0)))))))

(fn ConstructionScript)

(fn Interact
  (Variables|Default|SetGrabbing true)
  (return 0))